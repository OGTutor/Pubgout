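; Playable hero character Quin for a shooter, handling movement, look, aim-down-sights, firing and pause input.
; After a start delay it caches the local controller's HUD, which is hidden or shown as the game instance toggles pause.
; ADS is set locally and sent from clients by server event, while possession disables input.
; Firing plays muzzle effects and runs a debug-drawn muzzle line trace whose hit goes unused.
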(event `self.ReceiveBeginPlay`
  (`KismetSystemLibrary.Delay` 2.0)
  (if (`self.IsLocallyControlled`)
    (bind _asbp_shooter_player_controller (cast `/Game/Framework/BP_SHooter_PlayerController` (`GameplayStatics.GetPlayerController` 0)))
    (set `self.WB Ingame HUD` (`/Game/Framework/BP_SHooter_PlayerController.WB_IngameHUD` _asbp_shooter_player_controller))))

(event `InputAction|PauseGame`
  (params (Key :type "Key Structure"))
  (:`Pressed`
    (bind _asbp_shooter_gameinstance (cast `/Game/Framework/BP_SHooter_Gameinstance` (`GameplayStatics.GetGameInstance`)))
    (bind _isgamepausedresult (`/Game/Framework/BP_SHooter_Gameinstance.TogglePauseGame` _asbp_shooter_gameinstance))
    (if _isgamepausedresult
      (`Widget.SetVisibility` (`self.WB Ingame HUD`) "Hidden")
      (else
        (`Widget.SetVisibility` (`self.WB Ingame HUD`) "Visible")))))

(event `self.ReceivePossessed`
  (params (NewController :type "Controller Object Reference"))
  (`self.DisableAllInput` (cast `PlayerController` NewController :!pure true)))

(event `DisableAllInput`
  (params (PlayerController :type "PlayerController Object Reference"))
  (`self.DisableInput` PlayerController))

(event `InputAxis|MoveForward`
  (params (AxisValue :type "Float (single-precision)"))
  (`self.AddMovementInput` (`self.GetActorForwardVector`) AxisValue))

(event `InputAxis|Turn`
  (params (AxisValue :type "Float (single-precision)"))
  (`self.AddControllerYawInput` AxisValue))

(event `InputAxis|MoveRight`
  (params (AxisValue :type "Float (single-precision)"))
  (`self.AddMovementInput` (`self.GetActorRightVector`) AxisValue))

(event `InputAxis|LookUp`
  (params (AxisValue :type "Float (single-precision)"))
  (`self.AddControllerPitchInput` AxisValue))

(event `Svr_SetIsAds`
  (params (IsADS :type Boolean))
  (set `self.IsADS` IsADS))

(event `InputAction|ADS`
  (params (Key :type "Key Structure"))
  (:`Pressed`
    (`/Engine/EditorBlueprintResources/ActorMacros.Switch Has Authority`
      (:`Authority`
        _)
      (:`Remote`
        (`self.Svr_SetIsAds` true)))
    (set `self.IsADS` true))
  (:`Released`
    (`/Engine/EditorBlueprintResources/ActorMacros.Switch Has Authority`
      (:`Authority`
        _)
      (:`Remote`
        (`self.Svr_SetIsAds` false)))
    (set `self.IsADS` false)))

(event `InputAction|FireWeapon`
  (params (Key :type "Key Structure"))
  (bind (_returnvalue_location _returnvalue_rotation) (`KismetMathLibrary.BreakTransform` (`SceneComponent.GetSocketTransform` (`self.WeaponMesh`) "Muzzle" "RTS_World")))
  (:`Pressed`
    (`GameplayStatics.SpawnEmitterAttached` "/Game/MilitaryWeapSilver/FX/P_Pistol_MuzzleFlash_01.P_Pistol_MuzzleFlash_01" (`self.WeaponMesh`) "Muzzle" (0.0 0.0 0.0) (struct) (1.0 1.0 1.0) "SnapToTarget")
    (`GameplayStatics.PlaySound2D` "/Game/MilitaryWeapSilver/Sound/Pistol/Cues/PistolA_Fire_Cue.PistolA_Fire_Cue" 1.0 1.0 0.0 null null)
    (`KismetSystemLibrary.LineTraceSingle` :`Start` _returnvalue_location :`End` (+ _returnvalue_location (* (`KismetMathLibrary.GetForwardVector` _returnvalue_rotation) 100000)) :`TraceChannel` "TraceTypeQuery1" :`DrawDebugType` "ForDuration")))

(fn `UserConstructionScript`)